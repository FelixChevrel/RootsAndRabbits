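; Death manager actor for the rabbit game that handles falls into its kill box and runs the round countdown.
; A looping timer saves the player's last grounded location, and overlapping the box returns the player above it with zero velocity and gravity.
; Ingredients that enter the box are destroyed.
; A game-length timer feeds TimeRemaining every second and a countdown widget is created with this actor as owner, but EndGame is empty.
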(event OnComponentBeginOverlap(Box)
  (params (OverlappedComponent :type Primitive%20Component%20Object%20Reference) (OtherActor :type Actor%20Object%20Reference) (OtherComp :type Primitive%20Component%20Object%20Reference) (OtherBodyIndex :type Integer) (bFromSweep :type Boolean) (SweepResult :type Hit%20Result%20Structure%20%28by%20ref%29))
  (if (== OtherActor (Variables|Default|GetPlayer))
    (CallFunction|DEATH)
    (else
      (bind _asbp_ingredient (Utilities|Casting|CastToBP_ingredient OtherActor))
      (Actor|DestroyActor _asbp_ingredient))))

(event Custom|CheckLastPostion
  (bind _player (Variables|Default|GetPlayer))
  (if (AI|Components|NavMovement|IsMovingonGround (Variables|/Script/Engine.Character|GetCharacterMovement _player))
    (Variables|Default|SetSavedLocation (Transformation|GetActorLocation _player))))

(event Custom|DEATH
  (bind _player (Variables|Default|GetPlayer))
  (bind _charactermovement (Variables|/Script/Engine.Character|GetCharacterMovement _player))
  (Transformation|SetActorLocation _player (+ (Variables|Default|GetSavedLocation) "0,0,100.000000") false false)
  (Variables|/Script/Engine.MovementComponent|SetVelocity _charactermovement "0, 0, 0")
  (Variables|/Script/Engine.CharacterMovementComponent|SetGravityScale _charactermovement 0.0))

(event Custom|EndGame)

(event Custom|Countdown
  (Variables|Default|SetTimeRemaining (Math|Float|Round (Utilities|Time|GetTimerRemainingTimebyHandle (Variables|Default|GetEndGameEvent)))))

(event EventBeginPlay
  (Utilities|Time|SetTimerbyEvent (delegate Custom|CheckLastPostion) 1.0 true)
  (bind _asbp_rabbit_character (Utilities|Casting|CastToBP_Rabbit_Character (Game|Player|GetPlayerPawn 0)))
  (Variables|Default|SetPlayer _asbp_rabbit_character)
  (bind _returnvalue (Utilities|Time|SetTimerbyEvent (delegate Custom|EndGame) (Variables|Default|GetGameLength)))
  (Variables|Default|SetEndGameEvent _returnvalue)
  (Utilities|Time|SetTimerbyEvent (delegate Custom|Countdown) 1.0 true)
  (bind _returnvalue_2 (UserInterface|CreateWidget "/Game/Widget/WBP_countdown.WBP_countdown_C"))
  (bind _output_get (Variables|Default|SetCountdownWidget _returnvalue_2))
  (UserInterface|Viewport|AddtoViewport _output_get 0)
  (Variables|/Game/Widget/WBP_countdown.WBP_countdown_C|SetOwner _output_get self)
  (Development|PrintString "Hello"))

(fn ConstructionScript)