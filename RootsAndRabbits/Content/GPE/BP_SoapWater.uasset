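; BP_SoapWater is a slippery zone that makes the rabbit player slide while inside its box.
; BeginPlay caches the player character and its default ground friction and walking braking deceleration.
; Overlapping the box lowers both values on the player's CharacterMovement, and leaving restores the cached defaults.
; The construction script scales the decal to the box's world scale, swapping X and Z to suit its projection axis.
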(event OnComponentBeginOverlap(Box)
  (params (OverlappedComponent :type Primitive%20Component%20Object%20Reference) (OtherActor :type Actor%20Object%20Reference) (OtherComp :type Primitive%20Component%20Object%20Reference) (OtherBodyIndex :type Integer) (bFromSweep :type Boolean) (SweepResult :type Hit%20Result%20Structure%20%28by%20ref%29))
  (bind _player (Variables|Default|GetPlayer))
  (bind _charactermovement (Variables|/Script/Engine.Character|GetCharacterMovement _player))
  (if (== OtherActor (Variables|Default|GetPlayer))
    (Variables|/Script/Engine.CharacterMovementComponent|SetGroundFriction _charactermovement 0.5)
    (Variables|/Script/Engine.CharacterMovementComponent|SetBrakingDecelerationWalking _charactermovement 64.0)))

(event OnComponentEndOverlap(Box)
  (params (OverlappedComponent :type Primitive%20Component%20Object%20Reference) (OtherActor :type Actor%20Object%20Reference) (OtherComp :type Primitive%20Component%20Object%20Reference) (OtherBodyIndex :type Integer))
  (bind _player (Variables|Default|GetPlayer))
  (bind _charactermovement (Variables|/Script/Engine.Character|GetCharacterMovement _player))
  (if (== OtherActor (Variables|Default|GetPlayer))
    (Variables|/Script/Engine.CharacterMovementComponent|SetGroundFriction _charactermovement (Variables|Default|GetDefaultGroundFriction))
    (Variables|/Script/Engine.CharacterMovementComponent|SetBrakingDecelerationWalking _charactermovement (Variables|Default|GetDefaultBrakingDeceleration))))

(event EventBeginPlay
  (bind _asbp_rabbit_character (Utilities|Casting|CastToBP_Rabbit_Character (Game|Player|GetPlayerPawn 0)))
  (bind _output_get (Variables|Default|SetPlayer _asbp_rabbit_character))
  (Variables|Default|SetDefaultGroundFriction (Variables|/Script/Engine.CharacterMovementComponent|GetGroundFriction (Variables|/Script/Engine.Character|GetCharacterMovement _output_get)))
  (Variables|Default|SetDefaultBrakingDeceleration (Variables|/Script/Engine.CharacterMovementComponent|GetBrakingDecelerationWalking (Variables|/Script/Engine.Character|GetCharacterMovement _output_get))))

(fn ConstructionScript
  (bind _box (Variables|Default|GetBox))
  (bind _returnvalue (Transformation|GetWorldScale _box))
  (Transformation|SetWorldScale3D (Variables|Default|GetDecal) (Math|Vector|MakeVector (.z _returnvalue) (.y _returnvalue) (.x _returnvalue))))