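; BP_Bumper is a bounce pad that launches the player's rabbit character upward when it hits the mesh.
; A player hit passes a DoOnce gate and plays the Deform timeline, which animates the mesh's Z scale.
; When the timeline finishes, it launches the character with Power as an overriding Z velocity, plays a sponge bounce sound and resets the gate.
; The finish branch is hardwired true, leaving the Box overlap check unused.
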(event OnComponentHit(StaticMesh)
  (params (HitComponent :type Primitive%20Component%20Object%20Reference) (OtherActor :type Actor%20Object%20Reference) (OtherComp :type Primitive%20Component%20Object%20Reference) (NormalImpulse :type Vector :default "0, 0, 0") (Hit :type Hit%20Result%20Structure%20%28by%20ref%29))
  (if (== OtherActor (Game|Player|GetPlayerPawn 0))
    (Utilities|FlowControl|DoOnce false :!label _label
      (:Completed
        (bind _newtrack_0 (Timeline|Deform PlayFromStart)
          (:Update
            (Transformation|SetWorldScale3D (Variables|Default|GetStaticMesh) (Math|Vector|MakeVector 1.0 1.0 _newtrack_0)))
          (:Finished
            (if true
              (bind _asbp_rabbit_character (Utilities|Casting|CastToBP_Rabbit_Character (Game|Player|GetPlayerPawn 0)))
              (Character|LaunchCharacter _asbp_rabbit_character (Math|Vector|MakeVector 0.0 0.0 (Variables|Default|GetPower)) false true)
              (Audio|PlaySound2D "/Game/Audio/Sponge_Bounce.Sponge_Bounce" 1.0 1.0 0.0 0 0)
              (goto _label Reset)
              (else
                (goto _label Reset)))))))))

(fn ConstructionScript)