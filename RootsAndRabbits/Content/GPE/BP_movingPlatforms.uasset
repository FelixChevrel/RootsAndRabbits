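; Moving platform actor that carries its static mesh back and forth along a spline while active.
; Tick advances a normalized distance scaled by the speed modifier, places the mesh on the spline without sweeping, and flips direction past either end.
; Turnon, Toggle and ShutDown events control the active state.
; The construction script snaps the spline component to the actor's location.
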(event EventTick
  (params (DeltaSeconds :type Float%20%28single-precision%29))
  (bind _movementpath (Variables|Default|GetMovementPath))
  (if (Variables|Default|GetisActive)
    (Variables|Default|SetDistanceAlongSpline (+ (Variables|Default|GetDistanceAlongSpline) (* DeltaSeconds (Math|Float|SelectFloat 1.0 -1.0 (Variables|Default|GetDirection1)) (Variables|Default|GetSpeedModifiers))))
    (Transformation|SetWorldLocation (Variables|Default|GetStaticMesh) (Spline|GetLocationatDistanceAlongSpline _movementpath (* (Spline|GetSplineLength _movementpath) (Variables|Default|GetDistanceAlongSpline)) "World") false false)
    (if (select (Variables|Default|GetDirection1) (> (Variables|Default|GetDistanceAlongSpline) 1.0) (< (Variables|Default|GetDistanceAlongSpline) 0.0))
      (Variables|Default|SetDirection1 (select (Variables|Default|GetDirection1) false true)))))

(event EventTurnon
  (Variables|Default|SetisActive true))

(event EventShutDown
  (Variables|Default|SetisActive false))

(event EventToggle
  (Variables|Default|SetisActive (not (Variables|Default|GetisActive))))

(fn ConstructionScript
  (Transformation|SetWorldLocation (Variables|Default|GetMovementPath) (Transformation|GetActorLocation) false false))