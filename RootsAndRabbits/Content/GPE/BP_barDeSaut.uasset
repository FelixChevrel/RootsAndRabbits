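; BP_barDeSaut is a jump bar gameplay element that the rabbit player character can hang from and let go of.
; BeginPlay caches the player pawn as BP_Rabbit_Character.
; AttachPlayer stops its velocity, disables gravity, registers the bar as CurrentPole and teleports it to the Cube's height, keeping X and Y.
; Lache restores gravity and clears the pole state; both events have no caller in this Blueprint.
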(event Custom|AttachPlayer
  (bind _player (Variables|Default|GetPlayer))
  (bind _returnvalue (Transformation|GetActorLocation _player))
  (bind _charactermovement (Variables|/Script/Engine.Character|GetCharacterMovement _player))
  (Variables|/Script/Engine.MovementComponent|SetVelocity _charactermovement "0, 0, 0")
  (Variables|/Script/Engine.CharacterMovementComponent|SetGravityScale _charactermovement 0.0)
  (Variables|/Game/Character/BP_Rabbit_Character.BP_Rabbit_Character_C|SetOnPole _player true)
  (Variables|/Game/Character/BP_Rabbit_Character.BP_Rabbit_Character_C|SetCurrentPole _player self)
  (Transformation|SetActorLocation (Variables|Default|GetPlayer) (Math|Vector|MakeVector (.x _returnvalue) (.y _returnvalue) (.z (Transformation|GetWorldLocation (Variables|Default|GetCube)))) false true))

(event Custom|Lache
  (bind _player (Variables|Default|GetPlayer))
  (Variables|/Script/Engine.CharacterMovementComponent|SetGravityScale (Variables|/Script/Engine.Character|GetCharacterMovement _player) 1.0)
  (Variables|/Game/Character/BP_Rabbit_Character.BP_Rabbit_Character_C|SetOnPole _player false)
  (Variables|/Game/Character/BP_Rabbit_Character.BP_Rabbit_Character_C|SetCurrentPole _player 0))

(event EventBeginPlay
  (bind _asbp_rabbit_character (Utilities|Casting|CastToBP_Rabbit_Character (Game|Player|GetPlayerPawn 0)))
  (Variables|Default|SetPlayer _asbp_rabbit_character))

(fn ConstructionScript)