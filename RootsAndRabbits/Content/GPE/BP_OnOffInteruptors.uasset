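; A switch actor that toggles linked actors when a physics-simulating component overlaps its box trigger.
; Each hit calls ToggleMessage on every actor in ActorArray, then flips StateOn by swapping two cubes' visibility and the third cube's material.
; A DoOnce reset after a half-second delay debounces repeated hits.
; It plays a button click, or the Sonette sound instead when the actor carries that tag.
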(event OnComponentBeginOverlap(Box)
  (params (OverlappedComponent :type Primitive%20Component%20Object%20Reference) (OtherActor :type Actor%20Object%20Reference) (OtherComp :type Primitive%20Component%20Object%20Reference) (OtherBodyIndex :type Integer) (bFromSweep :type Boolean) (SweepResult :type Hit%20Result%20Structure%20%28by%20ref%29))
  (if (Physics|IsSimulatingPhysics OtherComp "None")
    (Utilities|FlowControl|DoOnce false :!label _label
      (:Completed
        (Utilities|FlowControl|Sequence
          (:then_0
            (for _array_element (Variables|Default|GetActorArray)
              (Class|BPIonOff|Toggle(Message) _array_element)))
          (:then_1
            (if (Variables|Default|GetstateOn)
              (Rendering|SetVisibility (Variables|Default|GetCube2) false false)
              (Rendering|Material|SetMaterial (Variables|Default|GetCube) 0 "/Engine/MapTemplates/Materials/BasicAsset01.BasicAsset01")
              (Rendering|SetVisibility (Variables|Default|GetCube1) true false)
              (if (Actor|ActorHasTag "Sonette")
                (Audio|PlaySoundatLocation "/Game/Audio/Sonette.Sonette" (Transformation|GetActorLocation) "0, 0, 0" 1.0 1.0 0.0 0 0 0 0)
                (Variables|Default|SetstateOn false)
                (else
                  (Audio|PlaySoundatLocation "/Game/Audio/Button_On.Button_On" (Transformation|GetActorLocation) "0, 0, 0" 1.0 1.0 0.0 0 0 0 0)
                  (Variables|Default|SetstateOn false)))
              (else
                (Rendering|SetVisibility (Variables|Default|GetCube2) true false)
                (Rendering|Material|SetMaterial (Variables|Default|GetCube) 0 "/Engine/MapTemplates/Materials/BasicAsset03.BasicAsset03")
                (Rendering|SetVisibility (Variables|Default|GetCube1) false false)
                (if (Actor|ActorHasTag "Sonette")
                  (Audio|PlaySoundatLocation "/Game/Audio/Sonette.Sonette" (Transformation|GetActorLocation) "0, 0, 0" 1.0 1.0 0.0 0 0 0 0)
                  (Variables|Default|SetstateOn true)
                  (else
                    (Audio|PlaySoundatLocation "/Game/Audio/Button_On.Button_On" (Transformation|GetActorLocation) "0, 0, 0" 1.0 1.0 0.0 0 0 0 0)
                    (Variables|Default|SetstateOn true))))))
          (:then_2
            (Utilities|FlowControl|Delay 0.5)
            (goto _label Reset)))))))

(event EventBeginPlay)

(event Collision|EventActorBeginOverlap
  (params (OtherActor :type Actor%20Object%20Reference)))

(event EventTick
  (params (DeltaSeconds :type Float%20%28single-precision%29)))

(fn ConstructionScript)