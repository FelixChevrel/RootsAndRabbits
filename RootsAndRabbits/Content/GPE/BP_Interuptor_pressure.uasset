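; Pressure plate switch that activates linked actors while the player or a physics object rests on it.
; Overlapping physics objects have their velocity zeroed and snap to the Arrow's position, then register as weight like the player.
; While the weight list is occupied, the plate turns green, sinks via a timeline, and sends turn-on messages to affected actors.
; Emptying the list sends shut-down messages, turns it red and reverses the timeline.
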(event OnComponentBeginOverlap(Box)
  (params (OverlappedComponent :type Primitive%20Component%20Object%20Reference) (OtherActor :type Actor%20Object%20Reference) (OtherComp :type Primitive%20Component%20Object%20Reference) (OtherBodyIndex :type Integer) (bFromSweep :type Boolean) (SweepResult :type Hit%20Result%20Structure%20%28by%20ref%29))
  (if (== OtherActor (Game|Player|GetPlayerPawn 0))
    (Utilities|Array|AddUnique (Variables|Default|GetWeightedObject) OtherActor :!label _label)
    (CallFunction|TurnonandOff true)
    (Rendering|Material|SetMaterial (Variables|Default|GetCube) 0 "/Game/Material/MAT_PH_Green_Inst.MAT_PH_Green_Inst")
    (bind _newtrack_0 (Timeline|Toggle Play)
      (:Update
        (Transformation|SetRelativeLocation (Variables|Default|GetCube) (Math|Vector|MakeVector 0.0 0.0 (* _newtrack_0 -25.0)) false false)))
    (elif (Physics|IsSimulatingPhysics OtherComp "None")
      (Physics|SetPhysicsLinearVelocity OtherComp "0, 0, 0" false "None")
      (Transformation|SetWorldLocation OtherComp (Transformation|GetWorldLocation (Variables|Default|GetArrow)) false false)
      (goto _label))))

(event OnComponentEndOverlap(Box)
  (params (OverlappedComponent :type Primitive%20Component%20Object%20Reference) (OtherActor :type Actor%20Object%20Reference) (OtherComp :type Primitive%20Component%20Object%20Reference) (OtherBodyIndex :type Integer))
  (bind _weightedobject (Variables|Default|GetWeightedObject))
  (Utilities|Array|RemoveItem _weightedobject OtherActor)
  (if (== (Utilities|Array|Length _weightedobject) 0)
    (CallFunction|TurnonandOff false)
    (Rendering|Material|SetMaterial (Variables|Default|GetCube) 0 "/Game/Material/MAT_PH_Red_Inst.MAT_PH_Red_Inst")
    (bind _newtrack_0 (Timeline|Toggle Reverse)
      (:Update
        (Transformation|SetRelativeLocation (Variables|Default|GetCube) (Math|Vector|MakeVector 0.0 0.0 (* _newtrack_0 -25.0)) false false)))))

(event Custom|TurnOnAndOff
  (params (On :type Boolean))
  (bind _actoraffected (Variables|Default|GetActorAffected))
  (if On
    (for _array_element _actoraffected
      (Class|BPIonOff|Turnon(Message) _array_element))
    (else
      (for _array_element_2 _actoraffected
        (Class|BPIonOff|ShutDown(Message) _array_element_2)))))

(fn ConstructionScript)