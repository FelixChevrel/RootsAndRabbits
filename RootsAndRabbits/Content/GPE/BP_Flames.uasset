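; BP_Flames is an animated flame hazard that sends the player rabbit back to safety on contact.
; A self-restarting timeline continuously animates the flame mesh's Z scale.
; A one-second looping timer records the player's location while they are moving on the ground.
; Sphere overlap teleports the player just above that saved location, zeroing velocity and gravity scale, which this Blueprint never restores.
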(event OnComponentBeginOverlap(Sphere)
  (params (OverlappedComponent :type Primitive%20Component%20Object%20Reference) (OtherActor :type Actor%20Object%20Reference) (OtherComp :type Primitive%20Component%20Object%20Reference) (OtherBodyIndex :type Integer) (bFromSweep :type Boolean) (SweepResult :type Hit%20Result%20Structure%20%28by%20ref%29))
  (if (== OtherActor (Variables|Default|GetPlayer))
    (CallFunction|DEATH)))

(event Custom|CheckLastPostion
  (bind _player (Variables|Default|GetPlayer))
  (if (AI|Components|NavMovement|IsMovingonGround (Variables|/Script/Engine.Character|GetCharacterMovement _player))
    (Variables|Default|SetSavedLocation (Transformation|GetActorLocation _player))))

(event Custom|DEATH
  (bind _player (Variables|Default|GetPlayer))
  (bind _charactermovement (Variables|/Script/Engine.Character|GetCharacterMovement _player))
  (Transformation|SetActorLocation _player (+ (Variables|Default|GetSavedLocation) "0,0,100.000000") false false)
  (Variables|/Script/Engine.MovementComponent|SetVelocity _charactermovement "0, 0, 0")
  (Variables|/Script/Engine.CharacterMovementComponent|SetGravityScale _charactermovement 0.0))

(event Custom|FlamesMove
  (bind _staticmesh (Variables|Default|GetStaticMesh))
  (bind _relativescale3d (Variables|/Script/Engine.SceneComponent|GetRelativeScale3D _staticmesh))
  (bind _newtrack_0 (Timeline|FlamesMovement PlayFromStart)
    (:Update
      (Transformation|SetRelativeScale3D _staticmesh (Math|Vector|MakeVector (.x _relativescale3d) (.y _relativescale3d) _newtrack_0)))
    (:Finished
      (CallFunction|FlamesMove))))

(event EventBeginPlay
  (bind _asbp_rabbit_character (Utilities|Casting|CastToBP_Rabbit_Character (Game|Player|GetPlayerPawn 0)))
  (Variables|Default|SetPlayer _asbp_rabbit_character)
  (CallFunction|FlamesMove)
  (Utilities|Time|SetTimerbyEvent (delegate Custom|CheckLastPostion) 1.0 true))

(fn ConstructionScript)