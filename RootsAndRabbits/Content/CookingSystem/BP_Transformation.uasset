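; BP_Transformation is a cooking utensil, such as a pan or blender, that transforms neutral ingredients into its ConvertType.
; On capsule overlap it snaps the ingredient to the Arrow, damps its velocity and calls Transform, passing itself.
; Actor tags pick the feedback: smoke for Pan, a temporarily shown cylinder for Blender.
; Throw launches an ingredient along the Arrow; ConvertType sets impulse strength and capsule height.
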(event OnComponentBeginOverlap(Capsule)
  (params (OverlappedComponent :type Primitive%20Component%20Object%20Reference) (OtherActor :type Actor%20Object%20Reference) (OtherComp :type Primitive%20Component%20Object%20Reference) (OtherBodyIndex :type Integer) (bFromSweep :type Boolean) (SweepResult :type Hit%20Result%20Structure%20%28by%20ref%29))
  (bind _cylinder (Variables|Default|GetCylinder))
  (bind _asbp_ingredient (Utilities|Casting|CastToBP_ingredient OtherActor)
    (:then
      (if (Utilities|Enum|Equal(Enum) (Variables|/Game/CookingSystem/BP_ingredient.BP_ingredient_C|GetState _asbp_ingredient) "NewEnumerator0")
        (bind _returnvalue (Physics|GetPhysicsLinearVelocity (Variables|/Game/CookingSystem/BP_ingredient.BP_ingredient_C|GetStaticMesh _asbp_ingredient) "None"))
        (Transformation|SetWorldLocation (Variables|/Game/CookingSystem/BP_ingredient.BP_ingredient_C|GetStaticMesh _asbp_ingredient) (Transformation|GetWorldLocation (Variables|Default|GetArrow)) false false)
        (Physics|SetPhysicsLinearVelocity (Variables|/Game/CookingSystem/BP_ingredient.BP_ingredient_C|GetStaticMesh _asbp_ingredient) (* _returnvalue "0.100000,0.100000,0.100000") false "None")
        (Default|Transform _asbp_ingredient (Variables|Default|GetConvertType) self)
        (if (Actor|ActorHasTag "Pan")
          (Development|PrintString "Pan")
          (Niagara|SpawnSystematLocation "/Game/Niagara/FX_Smoke.FX_Smoke" (Transformation|GetActorLocation))
          (elif (Actor|ActorHasTag "Blender")
            (Development|PrintString "Blender")
            (Development|SetHiddeninGame _cylinder false false)
            (Utilities|FlowControl|Delay 4.5)
            (Development|SetHiddeninGame _cylinder true false)))))
    (:CastFailed
      (Utilities|Casting|CastToBP_Rabbit_Character OtherActor))))

(event Custom|Throw
  (params (Ingredient :type BP%20Ingredient%20Object%20Reference))
  (Physics|AddImpulse (Variables|/Game/CookingSystem/BP_ingredient.BP_ingredient_C|GetStaticMesh Ingredient) (* (Math|Vector|GetForwardVector (Variables|Default|GetArrow)) (Utilities|Select :Index (Variables|Default|GetConvertType) :NewEnumerator0 0.0 :NewEnumerator1 1.25e+03 :NewEnumerator2 1e+03)) "None" true))

(fn ConstructionScript
  (Components|Capsule|SetCapsuleHalfHeight (Variables|Default|GetCapsule) (Utilities|Select :Index (Variables|Default|GetConvertType) :NewEnumerator0 0.0 :NewEnumerator1 3e+02 :NewEnumerator2 2e+02) true))