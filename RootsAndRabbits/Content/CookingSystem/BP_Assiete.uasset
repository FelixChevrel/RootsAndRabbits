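; Cooking plate that collects prepared ingredients and judges the dish they form against the game's recipe book.
; Non-neutral ingredients entering the sphere lose most horizontal velocity and add a unique type-and-state integer code to CurrentRecipe.
; Toggle sums the codes into a key for GI_Data's recipe book, printing and unlocking a match or printing "DISGUSTING!".
; It then calls DeathPending on overlapping ingredients, but never clears CurrentRecipe.
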(event OnComponentBeginOverlap(Sphere)
  (params (OverlappedComponent :type Primitive%20Component%20Object%20Reference) (OtherActor :type Actor%20Object%20Reference) (OtherComp :type Primitive%20Component%20Object%20Reference) (OtherBodyIndex :type Integer) (bFromSweep :type Boolean) (SweepResult :type Hit%20Result%20Structure%20%28by%20ref%29))
  (bind _asbp_ingredient (Utilities|Casting|CastToBP_ingredient OtherActor))
  (if (not (Utilities|Enum|Equal(Enum) (Variables|/Game/CookingSystem/BP_ingredient.BP_ingredient_C|GetState _asbp_ingredient) "NewEnumerator0"))
    (bind _returnvalue (Physics|GetPhysicsLinearVelocity (Variables|/Game/CookingSystem/BP_ingredient.BP_ingredient_C|GetStaticMesh _asbp_ingredient) "None"))
    (Physics|SetPhysicsLinearVelocity (Variables|/Game/CookingSystem/BP_ingredient.BP_ingredient_C|GetStaticMesh _asbp_ingredient) (* _returnvalue "0.100000,0.100000,1.000000") false "None")
    (Utilities|Array|AddUnique (Variables|Default|GetCurrentRecipe) (+ (* (Utilities|Select :Index (Variables|/Game/CookingSystem/BP_ingredient.BP_ingredient_C|GetType _asbp_ingredient) :NewEnumerator0 1 :NewEnumerator1 2 :NewEnumerator2 3) (Math|Integer|SelectInt 3 1 (== (Utilities|Select :Index (Variables|/Game/CookingSystem/BP_ingredient.BP_ingredient_C|GetState _asbp_ingredient) :NewEnumerator0 0 :NewEnumerator1 10 :NewEnumerator2 30) 30))) (Utilities|Select :Index (Variables|/Game/CookingSystem/BP_ingredient.BP_ingredient_C|GetState _asbp_ingredient) :NewEnumerator0 0 :NewEnumerator1 10 :NewEnumerator2 30)))))

(event EventBeginPlay
  (bind _asgi_data (Utilities|Casting|CastToGI_Data (Game|GetGameInstance)))
  (bind _output_get (Variables|Default|SetGameInstance _asgi_data))
  (bind _keys (Utilities|Map|Keys (Variables|/Game/SavedData/GI_Data.GI_Data_C|GetRecipeBookName _output_get)))
  (for _array_element _keys
    (Development|PrintString (Utilities|String|ToString(Integer) _array_element))))

(event EventToggle
  (bind _gameinstance (Variables|Default|GetGameInstance))
  (Variables|Default|SetRecipIndex 0)
  (for _array_element (Variables|Default|GetCurrentRecipe)
    (Variables|Default|SetRecipIndex (+ (Variables|Default|GetRecipIndex) _array_element)))
  (Development|PrintString (Utilities|String|ToString(Integer) (Variables|Default|GetRecipIndex)))
  (if (.ReturnValue (Utilities|Map|Find (Variables|/Game/SavedData/GI_Data.GI_Data_C|GetRecipeBookName _gameinstance) (Variables|Default|GetRecipIndex)))
    (Development|PrintString (.Value (Utilities|Map|Find (Variables|/Game/SavedData/GI_Data.GI_Data_C|GetRecipeBookName _gameinstance) (Variables|Default|GetRecipIndex))) true true "(R=0.139804,G=1.000000,B=0.000000,A=1.000000)" 3e+01)
    (Utilities|Map|Add (Variables|/Game/SavedData/GI_Data.GI_Data_C|GetRecipeBookAccess _gameinstance) (Variables|Default|GetRecipIndex) true)
    (else
      (Development|PrintString "DISGUSTING!" true true "(R=1.000000,G=0.000000,B=0.039932,A=1.000000)" 3e+01)))
  (for _array_element_2 (Collision|GetOverlappingActors (Variables|Default|GetSphere) "/Game/CookingSystem/BP_ingredient.BP_ingredient_C" :!class /Script/Engine.PrimitiveComponent)
    (bind _asbp_ingredient (Utilities|Casting|CastToBP_ingredient _array_element_2))
    (Default|DeathPending _asbp_ingredient)))

(fn ConstructionScript)