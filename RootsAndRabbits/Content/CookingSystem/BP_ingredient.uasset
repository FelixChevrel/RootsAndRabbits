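; BP_ingredient is a cooking ingredient that a utensil can transform into a mixed or roasted state.
; Transform plays a timeline for the requested goal, then sets the new State and has the utensil Throw the ingredient.
; Only roasting animates the look, driving RoastedValue on a dynamic material instance.
; The construction script creates that instance by ingredient Type, though all three types currently use the carrot material.
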(event Custom|Transform
  (params (transformationGoal :type State%20Enum :default "NewEnumerator0") (CookingUstensil :type BP%20Transformation%20Object%20Reference))
  (Variables|Default|SetCooking%20Ustensil CookingUstensil)
  (switch Utilities|FlowControl|Switch|SwitchonState transformationGoal
    (:NewEnumerator1
      (Timeline|MixedTimeline PlayFromStart
        (:Finished
          (Variables|Default|SetState "NewEnumerator1")
          (Default|Throw (Variables|Default|GetCooking%20Ustensil) self))))
    (:NewEnumerator2
      (bind _newtrack_0 (Timeline|RoastedTimeline PlayFromStart)
        (:Update
          (Rendering|Material|SetScalarParameterValue (Variables|Default|GetColorMaterial) "RoastedValue" _newtrack_0 :!class /Script/Engine.MaterialInstanceDynamic))
        (:Finished
          (Variables|Default|SetState "NewEnumerator2")
          (Default|Throw (Variables|Default|GetCooking%20Ustensil) self))))))

(fn ConstructionScript
  (bind _returnvalue (Rendering|Material|CreateDynamicMaterialInstance (Variables|Default|GetStaticMesh) 0 (Utilities|Select :Index (Variables|Default|GetType) :NewEnumerator0 "/Game/Material/MatCarrotMaterial.MatCarrotMaterial" :NewEnumerator1 "/Game/Material/MatCarrotMaterial.MatCarrotMaterial" :NewEnumerator2 "/Game/Material/MatCarrotMaterial.MatCarrotMaterial") "None" :!class /Script/Engine.PrimitiveComponent))
  (Variables|Default|SetColorMaterial _returnvalue))