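; BP_Spawner is an ingredient dispenser for the cooking system that keeps its configured IngredientType available in the level.
; A looping timer scans all BP_ingredient actors and, when none match that type, spawns one at the Arrow.
; The new ingredient's mesh gets a velocity-change impulse along the Arrow's forward vector to launch it out.
; The construction script picks the spawner's mesh from IngredientType; random-yaw nodes are left unconnected.
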(event Custom|Spawncheck
  (Variables|Default|SetSpawn? true)
  (bind _outactors (Actor|GetAllActorsOfClass "/Game/CookingSystem/BP_ingredient.BP_ingredient_C"))
  (for _array_element _outactors
    (if (Utilities|Enum|Equal(Enum) (Variables|/Game/CookingSystem/BP_ingredient.BP_ingredient_C|GetType _array_element) (Variables|Default|GetIngredientType))
      (Variables|Default|SetSpawn? false)))
  (if (Variables|Default|GetSpawn?)
    (bind _returnvalue (Game|SpawnActorfromClass "/Game/CookingSystem/BP_ingredient.BP_ingredient_C" (Math|Transform|MakeTransform (Transformation|GetWorldLocation (Variables|Default|GetArrow)) "0, 0, 0" "1.000000,1.000000,1.000000") "Undefined" 0 (Variables|Default|GetIngredientType) "NewEnumerator0" 0))
    (Physics|AddImpulse (Variables|/Game/CookingSystem/BP_ingredient.BP_ingredient_C|GetStaticMesh _returnvalue) (* (Math|Vector|GetForwardVector (Variables|Default|GetArrow)) 6.5e+02) "None" true)))

(event EventBeginPlay
  (Utilities|Time|SetTimerbyEvent (delegate Custom|Spawncheck) 5.0 true))

(fn ConstructionScript
  (Components|StaticMesh|SetStaticMesh (Variables|Default|GetCube) (Utilities|Select :Index (Variables|Default|GetIngredientType) :Option%200 "/Game/Meshes/GPEs/GPE_SpawnPotato.GPE_SpawnPotato" :Option%201 "/Game/Meshes/GPEs/GPE_SpawnCarotte.GPE_SpawnCarotte" :Option%202 "/Game/Map/_GENERATED/mathieuayer/Box_1B01B45C.Box_1B01B45C")))