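; Player rabbit character with camera-relative movement, physics-object grabbing and throwing, and BP_barDeSaut pole interaction.
; Tick turns it toward its velocity and ramps gravity while airborne, with a brief zero-gravity hang at jump apex.
; A sphere trace attaches objects or poles; releasing grab throws held objects hard, while a one-second hold tosses them gently.
; It also loads and periodically autosaves via GI_Data, plays music and opens the cooking book menu.
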(event Custom|OnApex
  (Variables|Default|SetFloat true)
  (Variables|/Script/Engine.CharacterMovementComponent|SetGravityScale (Variables|Character|GetCharacterMovement) 0.0)
  (Utilities|FlowControl|Delay 0.066)
  (Variables|Default|SetFloat false)
  (Variables|/Script/Engine.CharacterMovementComponent|SetGravityScale (Variables|Character|GetCharacterMovement) 4.0))

(event Custom|Autosave
  (Default|SaveProgress (Variables|Default|GetGameInstance)))

(event EventBeginPlay
  (Character|BindEventtoOnReachedJumpApex (delegate Custom|OnApex))
  (bind _asgi_data (Utilities|Casting|CastToGI_Data (Game|GetGameInstance)))
  (bind _output_get (Variables|Default|SetGameInstance _asgi_data))
  (Default|LoadSave _output_get)
  (Utilities|Time|SetTimerbyEvent (delegate Custom|Autosave) 2e+01 true)
  (Audio|PlaySound2D "/Game/Music/SCUE_music.SCUE_music" 1.0 1.0 0.0 0 0))

(event EventTick
  (params (DeltaSeconds :type Float%20%28single-precision%29))
  (Utilities|FlowControl|Sequence
    (:then_0
      (if (not (Variables|Default|GetOnPole))
        (if (not (Variables|Default|GetFloat))
          (|GravityAdjustements DeltaSeconds))))
    (:then_1
      (|CharacterROtation))
    (:then_2
      (Utilities|FlowControl|Gate true :!label _label
        (:Exit
          (Variables|Default|SetWillThrow true)
          (bind _output_get (Variables|Default|SetThrowValue (Math|Float|Clamp(Float) (+ (Variables|Default|GetThrowValue) DeltaSeconds))))
          (if (== _output_get 1.0)
            (Utilities|FlowControl|Sequence
              (:then_0
                (Transformation|DetachFromComponent (Variables|Default|GetHeldObject) "KeepWorld" "KeepWorld" "KeepWorld" true)
                (Physics|SetSimulatePhysics (Variables|Default|GetHeldObject) true)
                (Collision|SetCollisionEnabled (Variables|Default|GetHeldObject) "QueryAndPhysics")
                (Physics|AddImpulse (Variables|Default|GetHeldObject) (* (Transformation|GetActorForwardVector) 1e+02) "None" true)
                (Variables|Default|SetHeldObject 0)
                (Variables|Default|SetWillThrow false)
                (Variables|Default|SetHolding false))
              (:then_1
                (goto _label Close)))))))))

(event Input|ActionEvents|InputActionJump
  (params (Key :type Key%20Structure :default "None"))
  (:Pressed
    (if (Variables|Default|GetOnPole)
      (Character|LaunchCharacter "0, 0,1000.000000" false false)
      (Variables|Default|SetOnPole false)
      (else
        (Variables|Default|SetThrow true)
        (Variables|/Script/Engine.CharacterMovementComponent|SetbNotifyApex (Variables|Character|GetCharacterMovement) true)
        (Character|Jump))))
  (:Released
    (if (not (Variables|Default|GetOnPole))
      (Character|StopJumping)
      (Variables|/Script/Engine.CharacterMovementComponent|SetGravityScale (Variables|Character|GetCharacterMovement) 8.0))))

(event Input|ActionEvents|InputActionGrabAndLaunch
  (params (Key :type Key%20Structure :default "None"))
  (bind _arrow1 (Variables|Default|GetArrow1))
  (bind _charactermovement (Variables|Character|GetCharacterMovement))
  (bind _returnvalue (Transformation|GetWorldLocation _arrow1))
  (:Pressed
    (Variables|Default|SetThrowValue 0.0)
    (if (Variables|Default|GetOnPole)
      (Default|Lache (Variables|Default|GetCurrentPole))
      (elif (Variables|Default|GetHolding)
        (Variables|Default|SetWillThrow true)
        (Utilities|FlowControl|Gate true) ; enters at Open
        (else
          ;[1 1 1] Grab Object
          (bind (_outhit _returnvalue_2) (Collision|SphereTraceByChannel _returnvalue (+ _returnvalue (Math|Vector|SelectVector "0, 0,1.000000" (Math|Vector|ClampVectorSize (Variables|/Script/Engine.MovementComponent|GetVelocity _charactermovement) 0.0 5e+01) (AI|Components|NavMovement|IsMovingonGround _charactermovement))) 1e+02 "TraceTypeQuery3" false 0 "ForDuration"))
          (if _returnvalue_2
            (if (Physics|IsSimulatingPhysics (.HitComponent (Collision|BreakHitResult _outhit)) "None")
              (bind _output_get (Variables|Default|SetHeldObject (.HitComponent (Collision|BreakHitResult _outhit))))
              (Physics|SetSimulatePhysics _output_get false)
              (Transformation|AttachComponentToComponent _output_get (Variables|Default|GetHoldObject) "None" "SnapToTarget" "KeepWorld" "KeepWorld" false)
              (Collision|SetCollisionEnabled (Variables|Default|GetHeldObject) "NoCollision")
              (Variables|Default|SetHolding true)
              (else
                (bind _asbp_bar_de_saut (Utilities|Casting|CastToBP_barDeSaut (.HitActor (Collision|BreakHitResult _outhit))))
                (Default|AttachPlayer _asbp_bar_de_saut))))))))
  (:Released
    (if (Variables|Default|GetWillThrow)
      (Utilities|FlowControl|Sequence
        (:then_0
          (Utilities|FlowControl|Gate true) ; enters at Close
        )
        (:then_1
          (Variables|Default|SetThrow true)
          (Utilities|FlowControl|Delay 0.2)
          (Transformation|DetachFromComponent (Variables|Default|GetHeldObject) "KeepWorld" "KeepWorld" "KeepWorld" true)
          (Physics|SetSimulatePhysics (Variables|Default|GetHeldObject) true)
          (Collision|SetCollisionEnabled (Variables|Default|GetHeldObject) "QueryAndPhysics")
          (Physics|AddImpulse (Variables|Default|GetHeldObject) (* (Transformation|GetActorForwardVector) 1.25e+03) "None" true)
          (Variables|Default|SetHeldObject 0)
          (Variables|Default|SetWillThrow false)
          (Variables|Default|SetHolding false))))))

(event Input|ActionEvents|InputActionActivateMenu
  (params (Key :type Key%20Structure :default "None"))
  (:Pressed
    (Utilities|FlowControl|DoOnce false
      (:Completed
        (bind _returnvalue (UserInterface|CreateWidget "/Game/Widget/WBP_CookingBook.WBP_CookingBook_C"))
        (bind _output_get (Variables|Default|SetCookingBook _returnvalue))
        (UserInterface|Viewport|AddtoViewport _output_get 0)
        (Input|SetInputModeGameandUI (Game|GetPlayerController 0) _output_get "DoNotLock" true)))))

(event Input|AxisEvents|InputAxisForward
  (params (AxisValue :type Float%20%28single-precision%29))
  ;[1 1 1] Movements
  (Class|PawnMovementComponent|AddInputVector (Variables|Character|GetCharacterMovement) (* AxisValue (Math|Vector|Normalize (Math|Vector|ProjectVectorontoPlane (Math|Vector|GetForwardVector (Variables|Default|GetCamera)) "0, 0,1.000000")) (Math|Float|SelectFloat 0.0 1.0 (Variables|Default|GetOnPole))) false))

(event Input|AxisEvents|InputAxisRight
  (params (AxisValue :type Float%20%28single-precision%29))
  ;[1 1 1] Movements
  (Class|PawnMovementComponent|AddInputVector (Variables|Character|GetCharacterMovement) (* AxisValue (Math|Vector|Normalize (Math|Vector|ProjectVectorontoPlane (Math|Vector|GetRightVector (Variables|Default|GetCamera)) "0, 0,1.000000")) (Math|Float|SelectFloat 0.0 1.0 (Variables|Default|GetOnPole))) false))

(fn ConstructionScript)